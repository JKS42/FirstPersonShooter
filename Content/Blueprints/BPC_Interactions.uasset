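; BPC_Interactions is an actor component that handles interaction between its owner and nearby interactables, including item pickups.
; AddInteractables adds or removes entries in a unique list, and IA_Interact sends InteractMessage to the first entry, passing the owner.
; OnInteractedEvent switches on interaction type and, for the None type only, calls OnItemPickedUp with the item details.
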(event Input|EnhancedActionEvents|EnhancedInputActionIA_Interact
  (params (ActionValue :type Boolean) (ElapsedSeconds :type Float%20%28double-precision%29) (TriggeredSeconds :type Float%20%28double-precision%29) (InputAction :type Input%20Action%20Object%20Reference :default "/Game/Input/PlayerActions/IA_Interact.IA_Interact"))
  (bind _interactables (Variables|Default|GetInteractables))
  (:Started
    (if (> (Utilities|Array|Length _interactables) 0)
      (Class|BPIInteract|Interact(Message) (Utilities|Array|Get(acopy) _interactables) (Components|GetOwner)))))

(event EventAddInteractables
  (params (Add :type Boolean) (Interactable :type Actor%20Object%20Reference))
  (if Add
    (Utilities|Array|AddUnique (Variables|Default|GetInteractables) Interactable)
    (else
      (Utilities|Array|RemoveItem (Variables|Default|GetInteractables) Interactable))))

(event EventOnInteractedEvent
  (params (InteractType :type E_InteractType%20Enum :default "NewEnumerator0") (ItemDetails :type S%20Item%20Details%20Structure))
  (switch Utilities|FlowControl|Switch|SwitchonE_InteractType InteractType
    (:NewEnumerator1
      (Default|CallOnItemPickedUp ItemDetails))))