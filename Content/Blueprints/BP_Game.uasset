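; Game mode that handles respawning and keeps a shared player list with names and scores.
; It binds to the first BP_OnDeath actor's death event, which caches all BP_SpawnPoint actors.
; RespawnEnemy and RespawnPlayer spawn at a random cached point, and the player respawn is possessed by player controller 0.
; Login and logout update the controller array, then UpdateListGM rebuilds the list and pushes it to every BP_Controller.
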(event Custom|RespawnPlayer
  (params (Player :type Actor%20Object%20Reference))
  (bind _returnvalue (Game|SpawnActorfromClass "/Game/PlayerController/BP_BaseCharacter.BP_BaseCharacter_C" (Transformation|GetActorTransform (Utilities|Array|Get(acopy) (stale Custom|HandleDeath _outactors) (Math|Random|RandomIntegerinRange 0 (- (Utilities|Array|Length (stale Custom|HandleDeath _outactors)) 1)))) "Undefined" "MultiplyWithRoot" 0 0))
  (Pawn|Possess (Game|GetPlayerController 0) _returnvalue))

(event Custom|HandleDeath
  (bind _outactors (Actor|GetAllActorsOfClass "/Game/Spawn/BP_SpawnPoint.BP_SpawnPoint_C")))

(event Custom|RespawnEnemy
  (Game|SpawnActorfromClass "/Game/Enemy/BP_Enemy.BP_Enemy_C" (Transformation|GetActorTransform (Utilities|Array|Get(acopy) (stale Custom|HandleDeath _outactors) (Math|Random|RandomIntegerinRange 0 (- (Utilities|Array|Length (stale Custom|HandleDeath _outactors)) 1)))) "Undefined" "MultiplyWithRoot" 0 0))

(event EventPostLogin
  (params (NewPlayer :type Player%20Controller%20Object%20Reference))
  (Utilities|Array|Add (Variables|Default|GetAllPCs) NewPlayer)
  (CallFunction|UpdateListGM))

(event EventOnLogout
  (params (ExitingController :type Controller%20Object%20Reference))
  (bind _asplayer_controller (Utilities|Casting|CastToPlayerController ExitingController))
  (Utilities|Array|RemoveItem (Variables|Default|GetAllPCs) _asplayer_controller)
  (CallFunction|UpdateListGM))

(event EventBeginPlay
  (bind _outactors (Actor|GetAllActorsOfClass "/Game/Blueprints/BP_OnDeath.BP_OnDeath_C"))
  (EventDispatchers|BindEventtoOnDeathEvent (Utilities|Array|Get(acopy) _outactors) (delegate Custom|HandleDeath)))

(fn ConstructionScript)

(fn UpdateListGM
  (Utilities|Array|Clear (Variables|Default|GetPlayerList))
  (for _array_element (Variables|Default|GetAllPCs)
    (Utilities|Array|Add (Variables|Default|GetPlayerList) (Utilities|Struct|MakeS_Player (Utilities|Text|ToText(String) (PlayerState|GetPlayerName (Variables|/Script/Engine.Controller|GetPlayerState _array_element))) (Variables|/Game/PlayerController/BP_Controller.BP_Controller_C|GetScore (.AsBP%20Controller (Utilities|Casting|CastToBP_Controller _array_element))))))
  (for _array_element_2 (Variables|Default|GetAllPCs)
    (bind _asbp_controller (Utilities|Casting|CastToBP_Controller _array_element_2))
    (Default|UpdatePlayerlistPC _asbp_controller (Variables|Default|GetPlayerList))))