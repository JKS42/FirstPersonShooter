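; Base pickup actor Blueprint for an interactable item that is handed to whoever interacts with it.
; The construction script fills ItemDetails from the DataTableItem row when a table is set, then applies its PickUpMesh to the static mesh.
; On Interact, it sends ItemDetails through OnInteractedEventMessage to the interactor's "Player"-tagged component, then destroys itself.
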(event EventBeginPlay
  (|CallParentFunction) ; This node is disabled and will not be called.\nDrag off pins to build functionality.
)

(event Collision|EventActorBeginOverlap
  (params (OtherActor :type Actor%20Object%20Reference))
  (|CallParentFunction OtherActor) ; This node is disabled and will not be called.\nDrag off pins to build functionality.
)

(event EventTick
  (params (DeltaSeconds :type Float%20%28single-precision%29))
  (|CallParentFunction DeltaSeconds) ; This node is disabled and will not be called.\nDrag off pins to build functionality.
)

(event EventInteract
  (params (Interactor :type Actor%20Object%20Reference))
  (Class|BPIInteraction|OnInteractedEvent(Message) (Class|Actor|FindComponentbyTag Interactor "/Script/Engine.ActorComponent" "Player") "NewEnumerator1" (Variables|Default|GetItemDetails))
  (Actor|DestroyActor))

(fn ConstructionScript
  (bind _data_table_item (Variables|Default|GetData%20Table%20Item))
  (bind (_datatable _rowname) (Utilities|Struct|BreakDataTableRowHandle _data_table_item))
  (|CallParentFunction)
  (Utilities|IsValid _datatable
    (:Is%20Valid
      (bind _returnvalue (Utilities|GetDataTableRow _datatable _rowname)
        (:then
          (Variables|Default|SetItemDetails _returnvalue))))
    (:Is%20Not%20Valid
      _))
  (Components|StaticMesh|SetStaticMesh (Variables|Default|GetStaticMesh) (.PickUpMesh (Utilities|Struct|BreakS_ItemDetails (Variables|Default|GetItemDetails)))))