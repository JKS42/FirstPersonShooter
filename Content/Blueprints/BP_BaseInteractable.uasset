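; Base interactable actor that shows a prompt and registers itself with the player when the player character is in range.
; On BeginPlay, its widget component's text is set from the InteractType enum name.
; Sphere begin and end overlaps toggle widget visibility and send AddInteractables add or remove messages to the player's component tagged "Player", avoiding casts.
; The interaction response itself is not implemented here.
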(event OnComponentBeginOverlap(Sphere)
  (params (OverlappedComponent :type Primitive%20Component%20Object%20Reference) (OtherActor :type Actor%20Object%20Reference) (OtherComp :type Primitive%20Component%20Object%20Reference) (OtherBodyIndex :type Integer) (bFromSweep :type Boolean) (SweepResult :type Hit%20Result%20Structure%20%28by%20ref%29))
  (if (== OtherActor (Game|GetPlayerCharacter 0))
    (Class|BPIInteraction|AddInteractables(Message) (Class|Actor|FindComponentbyTag OtherActor "/Script/Engine.ActorComponent" "Player") true self)
    (Rendering|SetVisibility (Variables|Default|GetWidget) true false)))

(event OnComponentEndOverlap(Sphere)
  (params (OverlappedComponent :type Primitive%20Component%20Object%20Reference) (OtherActor :type Actor%20Object%20Reference) (OtherComp :type Primitive%20Component%20Object%20Reference) (OtherBodyIndex :type Integer))
  (if (== OtherActor (Game|GetPlayerCharacter 0))
    (Class|BPIInteraction|AddInteractables(Message) (Class|Actor|FindComponentbyTag OtherActor "/Script/Engine.ActorComponent" "Player") false self)
    (Rendering|SetVisibility (Variables|Default|GetWidget) false false)))

(event EventBeginPlay
  (Class|WBPWidgets|SetInteractionText(Message) (UserInterface|GetUserWidgetObject (Variables|Default|GetWidget)) (Utilities|Text|ToText(String) (Utilities|String|EnumtoString (Variables|Default|GetInteractType)))))

(event Collision|EventActorBeginOverlap
  (params (OtherActor :type Actor%20Object%20Reference)))

(event EventTick
  (params (DeltaSeconds :type Float%20%28single-precision%29)))

(fn ConstructionScript)