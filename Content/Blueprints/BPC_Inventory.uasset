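; BPC_Inventory is an actor component that stores items for its owning actor in an Inventory collection.
; Add and remove functions modify the collection directly, with no capacity or validity checks.
; Dropping removes the item, then spawns a BP_BasePickup at the owner's location carrying that item's details.
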(event EventBeginPlay)

(event EventTick
  (params (DeltaSeconds :type Float%20%28single-precision%29)))

(fn AddtoInventory
  (params (NewItem :type S%20Item%20Details%20Structure%20%28by%20ref%29))
  (Utilities|Array|Add (Variables|Default|GetInventory) NewItem))

(fn RemovefromInventory
  (params (Item :type S%20Item%20Details%20Structure%20%28by%20ref%29))
  (Utilities|Array|RemoveItem (Variables|Default|GetInventory) Item))

(fn DropfromInventory
  (params (ItemDetails :type S%20Item%20Details%20Structure%20%28by%20ref%29))
  (CallFunction|RemovefromInventory ItemDetails)
  (Game|SpawnActorfromClass :Class "/Game/Blueprints/BP_BasePickup.BP_BasePickup_C" :SpawnTransform (Math|Transform|MakeTransform (Transformation|GetActorLocation (Components|GetOwner)) "0, 0, 0" "1.000000,1.000000,1.000000") :CollisionHandlingOverride "Undefined" :TransformScaleMethod "MultiplyWithRoot" :ItemDetails ItemDetails :Instigator 0))