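; Player controller that sets up the local HUD and movement input and drives a score-tracking player list.
; BeginPlay adds the Enhanced Input movement context, creates the HUD for the local controller and sets game-only input.
; Holding Tab shows the list, while F increments Score and asks BP_Game to update it.
; List updates received through UpdatePlayerlistPC pass to the HUD, retrying on a short delay until the widget exists.
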(event Custom|UpdatePlayerlistPC
  (params (PlayerList :type Array%20of%20S%20Player%20Structures))
  (bind _ui_ref (Variables|Default|GetUI_Ref))
  (Utilities|IsValid _ui_ref :!label _label
    (:Is%20Valid
      (Default|UpdatePlayerlist _ui_ref PlayerList))
    (:Is%20Not%20Valid
      (Utilities|FlowControl|Delay 0.1)
      (goto _label))))

(event Custom|IncreaseScore
  (Math|Integer|IncrementInt (Variables|Default|GetScore)
    (:%20%20
      (bind _asbp_game (Utilities|Casting|CastToBP_Game (Game|GetGameMode)))
      (Default|UpdateListGM _asbp_game))))

(event EventBeginPlay
  (bind _returnvalue (Game|GetPlayerController 0))
  (bind _returnvalue_2 (Class|InputDeviceLibrary|GetPlayerControllerfromInputDevice (Class|InputDeviceLibrary|GetDefaultInputDevice)))
  (Utilities|IsValid (PlayerController|LocalPlayerSubsystems|GetEnhancedInputLocalPlayerSubsystem _returnvalue_2)
    (:Is%20Valid
      (Input|AddMappingContext (PlayerController|LocalPlayerSubsystems|GetEnhancedInputLocalPlayerSubsystem _returnvalue_2) "/Game/Input/IMC_Movement.IMC_Movement" 0 "(bIgnoreAllPressedKeysUntilRelease=True,bForceImmediately=False,bNotifyUserSettings=False)")
      (CallFunction|SetupUI)
      (Variables|/Script/Engine.PlayerController|SetbShowMouseCursor _returnvalue false)
      (Input|SetInputModeGameOnly _returnvalue false))))

(event Input|KeyboardEvents|Tab
  (params (Key :type Key%20Structure :default "None"))
  (bind _ui_ref (Variables|Default|GetUI_Ref))
  (:Pressed
    (Default|ShowPlayerList _ui_ref true))
  (:Released
    (Default|ShowPlayerList _ui_ref false)))

(event Input|KeyboardEvents|F
  (params (Key :type Key%20Structure :default "None"))
  (:Pressed
    (CallFunction|IncreaseScore)))

(fn ConstructionScript)

(fn SetupUI
  (if (Pawn|IsLocalController)
    (bind _returnvalue (UserInterface|CreateWidget "/Game/UI/WBP_HUD.WBP_HUD_C"))
    (bind _output_get (Variables|Default|SetUI_Ref _returnvalue))
    (UserInterface|Viewport|AddtoViewport _output_get 0)))