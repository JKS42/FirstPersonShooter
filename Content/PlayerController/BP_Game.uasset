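; BP_Game handles respawning of enemies and the player at random spawn points.
; Tick refreshes the list of all BP_SpawnPoint actors every frame, and both respawn events pick a random entry for the spawn transform.
; RespawnEnemy spawns a BP_Enemy there.
; RespawnPlayer spawns a BP_BaseCharacter and has player controller 0 possess it, ignoring its Player input.
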(event Custom|RespawnPlayer
  (params (Player :type Actor%20Object%20Reference))
  (bind _returnvalue (Game|SpawnActorfromClass "/Game/PlayerController/BP_BaseCharacter.BP_BaseCharacter_C" (Transformation|GetActorTransform (Utilities|Array|Get(acopy) (stale EventTick _outactors) (Math|Random|RandomIntegerinRange 0 (- (Utilities|Array|Length (stale EventTick _outactors)) 1)))) "Undefined" "MultiplyWithRoot" 0 0))
  (Pawn|Possess (Game|GetPlayerController 0) _returnvalue))

(event Custom|RespawnEnemy
  (Game|SpawnActorfromClass "/Game/Enemy/BP_Enemy.BP_Enemy_C" (Transformation|GetActorTransform (Utilities|Array|Get(acopy) (stale EventTick _outactors) (Math|Random|RandomIntegerinRange 0 (- (Utilities|Array|Length (stale EventTick _outactors)) 1)))) "Undefined" "MultiplyWithRoot" 0 0))

(event EventTick
  (params (DeltaSeconds :type Float%20%28single-precision%29))
  (bind _outactors (Actor|GetAllActorsOfClass "/Game/Spawn/BP_SpawnPoint.BP_SpawnPoint_C")))

(fn ConstructionScript)