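; Player character Blueprint handling movement, jumping, sprinting, montage-based aiming with a crosshair, health and weapons.
; BeginPlay creates health and ammo HUDs and attaches a semi-auto weapon, which receives fire input.
; Weapon keys spawn and destroy guns, with full-auto requiring a second-weapon flag; interact adds ammo or sphere-traces for interface targets.
; Damage updates health until death disables input, while custom events provide screen-centre bullet traces and physics hit impulses.
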(event Custom|SpawnWeapon
  (params (Weapon :type BP%20Base%20Weapon%20Class%20Reference))
  ;[0.15 0.15 0.15 0.5] Weapon Pickup
  (bind _returnvalue (Game|SpawnActorfromClass Weapon (Transformation|GetActorTransform) "Undefined" "MultiplyWithRoot" 0 0))
  (bind _output_get (Variables|Default|SetEquippedWeapon _returnvalue))
  (Transformation|AttachComponentToComponent _output_get (Variables|Character|GetMesh) "WeaponSocket" "SnapToTarget" "SnapToTarget" "SnapToTarget" true)
  (Variables|Default|SetHas2ndWeapon true))

(event Custom|BulletTrace
  (bind _returnvalue (Game|GetPlayerController 0))
  (bind (_sizex _sizey) (HUD|GetViewportSize _returnvalue))
  (bind _returnvalue_2 (/ _sizey 2))
  (bind _returnvalue_3 (/ _sizex 2))
  (bind _returnvalue_4 (Math|Conversions|ToFloat(Integer) _returnvalue_3))
  (bind _returnvalue_5 (Math|Conversions|ToFloat(Integer) _returnvalue_2))
  (bind (_worldlocation _worlddirection) (Class|PlayerController|DeprojectScreenPositiontoWorld _returnvalue _returnvalue_4 _returnvalue_5))
  ;[0.15 0.15 0.15 0.5] HitTrace
  (bind (_outhit _returnvalue_6) (Collision|LineTraceForObjects (+ _worldlocation (* _worlddirection 1e+01)) (+ _worldlocation (* _worlddirection 3e+03)) (Utilities|Array|MakeArray "ObjectTypeQuery4") false 0 "ForDuration"))
  (if _returnvalue_6
    (Variables|Default|SetBulletImpactLoc (.ImpactPoint (Collision|BreakHitResult _outhit)))
    (bind _output_get (Variables|Default|SetHitBoneName (.HitBoneName (Collision|BreakHitResult _outhit))))
    (Development|PrintText (Utilities|Text|ToText(Name) _output_get))
    (else
      (Variables|Default|SetBulletImpactLoc (.TraceEnd (Collision|BreakHitResult _outhit))))))

(event Custom|HitImpact
  (params (ForwardVector :type Vector) (RightVector :type Vector) (Impulse%20AMT :type Float%20%28double-precision%29) (Bone%20Name :type Name))
  (bind _mesh (Variables|Character|GetMesh))
  ;[0.15 0.15 0.15 0.5] Bullet Impact
  (Collision|SetCollisionEnabled _mesh "QueryAndPhysics")
  (Physics|SetSimulatePhysics _mesh true)
  (Physics|AddImpulse (Variables|Character|GetMesh) (* (Math|Vector|RotateVector ForwardVector (Math|Vector|RotatorfromAxisandAngle (Math|Vector|NegateVector RightVector) 0.0)) Impulse%20AMT) Bone%20Name true))

(event Input|EnhancedActionEvents|EnhancedInputActionIA_Sprinting
  (params (ActionValue :type Boolean) (ElapsedSeconds :type Float%20%28double-precision%29) (TriggeredSeconds :type Float%20%28double-precision%29) (InputAction :type Input%20Action%20Object%20Reference :default "/Game/Input/PlayerActions/IA_Sprinting.IA_Sprinting"))
  ;[0.15 0.15 0.15 0.5] Sprinting
  (:Triggered
    (CallFunction|Sprint))
  (:Completed
    (CallFunction|StopSprinting)))

(event Input|EnhancedActionEvents|EnhancedInputActionAI_Jump
  (params (ActionValue :type Boolean) (ElapsedSeconds :type Float%20%28double-precision%29) (TriggeredSeconds :type Float%20%28double-precision%29) (InputAction :type Input%20Action%20Object%20Reference :default "/Game/Input/PlayerActions/AI_Jump.AI_Jump"))
  ;[0.15 0.15 0.15 0.5] Jumping
  (:Triggered
    (Character|Jump)
    (Development|PrintText "Hello"))
  (:Completed
    (Character|StopJumping)))

(event Input|EnhancedActionEvents|EnhancedInputActionIA_MouseMovement
  (params (ActionValue :type Vector%202D%20Structure) (ElapsedSeconds :type Float%20%28double-precision%29) (TriggeredSeconds :type Float%20%28double-precision%29) (InputAction :type Input%20Action%20Object%20Reference :default "/Game/Input/PlayerActions/IA_MouseMovement.IA_MouseMovement"))
  (bind _returnvalue (Pawn|GetControlRotation :!class /Script/Engine.Pawn))
  ;[0.15 0.15 0.15 0.5] Camera
  (Pawn|Input|AddControllerYawInput (.x ActionValue))
  (Pawn|Input|AddControllerPitchInput (.y ActionValue))
  (Transformation|SetActorRotation (Math|Interpolation|RInterpTo (Transformation|GetActorRotation) (Math|Rotator|MakeRotator (.roll _returnvalue) (.pitch _returnvalue) (.yaw _returnvalue)) (stale EventTick DeltaSeconds) 2.5)))

(event Input|EnhancedActionEvents|EnhancedInputActionIA_Move
  (params (ActionValue :type Float%20%28double-precision%29) (ElapsedSeconds :type Float%20%28double-precision%29) (TriggeredSeconds :type Float%20%28double-precision%29) (InputAction :type Input%20Action%20Object%20Reference :default "/Game/Input/PlayerActions/IA_Move.IA_Move"))
  ;[0.15 0.15 0.15 0.5] Camera
  (Pawn|Input|AddMovementInput (Math|Vector|GetForwardVector (Math|Rotator|MakeRotator 0.0 0.0 (.yaw (Pawn|GetControlRotation :!class /Script/Engine.Pawn)))) ActionValue false))

(event Input|EnhancedActionEvents|EnhancedInputActionIA_MoveRight
  (params (ActionValue :type Float%20%28double-precision%29) (ElapsedSeconds :type Float%20%28double-precision%29) (TriggeredSeconds :type Float%20%28double-precision%29) (InputAction :type Input%20Action%20Object%20Reference :default "/Game/Input/PlayerActions/IA_MoveRight.IA_MoveRight"))
  ;[0.15 0.15 0.15 0.5] Strafe
  (Pawn|Input|AddMovementInput (Math|Vector|GetRightVector (Math|Rotator|MakeRotator 0.0 0.0 (.yaw (Pawn|GetControlRotation :!class /Script/Engine.Pawn)))) ActionValue false))

(event Input|EnhancedActionEvents|EnhancedInputActionIA_Interact
  (params (ActionValue :type Boolean) (ElapsedSeconds :type Float%20%28double-precision%29) (TriggeredSeconds :type Float%20%28double-precision%29) (InputAction :type Input%20Action%20Object%20Reference :default "/Game/Input/PlayerActions/IA_Interact.IA_Interact"))
  (bind _returnvalue (Transformation|GetActorLocation))
  (bind _fullauto (Variables|Default|GetFullAuto))
  ;[0.15 0.15 0.15 0.5] Weapon Pickup
  (if (Variables|Default|GetHas2ndWeapon)
    (Variables|/Game/Weapons/Weapons/BP_BaseWeapon.BP_BaseWeapon_C|SetAmmo (Variables|Default|GetFullAuto) (+ (Variables|/Game/Weapons/Weapons/BP_BaseWeapon.BP_BaseWeapon_C|GetAmmo _fullauto) (Variables|/Game/Weapons/Weapons/BP_BaseWeapon.BP_BaseWeapon_C|GetMaxAmmo _fullauto)))
    (else
      (bind (_outhits _returnvalue_2) (Collision|MultiSphereTraceForObjects _returnvalue _returnvalue 1.5e+02 (Utilities|Array|MakeArray "ObjectTypeQuery4") false 0 "None"))
      (if _returnvalue_2
        (bind _array_element (Utilities|Array|ForEachLoopwithBreak _outhits)
          (:LoopBody
            (if (Utilities|DoesObjectImplementInterface (.HitActor (Collision|BreakHitResult _array_element)) "/Game/Weapons/Interfaces/BPI_Interaction.BPI_Interaction_C")
              (Class|BPIInteraction|Interact(Message) (.HitActor (Collision|BreakHitResult _array_element)) self))))))))

(event Input|EnhancedActionEvents|EnhancedInputActionIA_Weapon1
  (params (ActionValue :type Boolean) (ElapsedSeconds :type Float%20%28double-precision%29) (TriggeredSeconds :type Float%20%28double-precision%29) (InputAction :type Input%20Action%20Object%20Reference :default "/Game/Input/PlayerActions/IA_Weapon1.IA_Weapon1"))
  ;[0.15 0.15 0.15 0.5] Weapon Switching
  (bind _returnvalue (Game|SpawnActorfromClass "/Game/Weapons/Weapons/BP_SemiAutoBaseWeapon.BP_SemiAutoBaseWeapon_C" (Transformation|GetActorTransform) "Undefined" "MultiplyWithRoot" 0 0))
  (bind _output_get (Variables|Default|SetEquippedWeapon _returnvalue))
  (Transformation|AttachComponentToComponent _output_get (Variables|Character|GetMesh) "WeaponSocket" "SnapToTarget" "SnapToTarget" "SnapToTarget" true)
  (Actor|DestroyActor (stale Input|EnhancedActionEvents|EnhancedInputActionIA_Weapon2 _returnvalue)))

(event Input|EnhancedActionEvents|EnhancedInputActionIA_Weapon2
  (params (ActionValue :type Boolean) (ElapsedSeconds :type Float%20%28double-precision%29) (TriggeredSeconds :type Float%20%28double-precision%29) (InputAction :type Input%20Action%20Object%20Reference :default "/Game/Input/PlayerActions/IA_Weapon2.IA_Weapon2"))
  ;[0.15 0.15 0.15 0.5] Weapon Switching
  (if (Variables|Default|GetHas2ndWeapon)
    (bind _returnvalue (Game|SpawnActorfromClass "/Game/Weapons/Weapons/BP_FullAutoBaseWeapon1.BP_FullAutoBaseWeapon1_C" (Transformation|GetActorTransform) "Undefined" "MultiplyWithRoot" 0 0))
    (bind _output_get (Variables|Default|SetEquippedWeapon _returnvalue))
    (Transformation|AttachComponentToComponent _output_get (Variables|Character|GetMesh) "WeaponSocket" "SnapToTarget" "SnapToTarget" "SnapToTarget" true)
    (Actor|DestroyActor (stale Input|EnhancedActionEvents|EnhancedInputActionIA_Weapon1 _returnvalue))))

(event Input|EnhancedActionEvents|EnhancedInputActionIA_Fire
  (params (ActionValue :type Boolean) (ElapsedSeconds :type Float%20%28double-precision%29) (TriggeredSeconds :type Float%20%28double-precision%29) (InputAction :type Input%20Action%20Object%20Reference :default "/Game/Input/PlayerActions/IA_Fire.IA_Fire"))
  (:Started
    (Default|Shoot (Variables|Default|GetEquippedWeapon)))
  (:Completed
    (Default|EndShoot (Variables|Default|GetEquippedWeapon))))

(event Game|Damage|EventAnyDamage
  (params (Damage :type Float%20%28single-precision%29) (DamageType :type Damage%20Type%20Object%20Reference) (InstigatedBy :type Controller%20Object%20Reference) (DamageCauser :type Actor%20Object%20Reference))
  ;[0.15 0.15 0.15 0.5] Player health
  (if (not (Variables|Default|GetisDead))
    (bind _output_get (Variables|Default|SetCurrentHealth (Math|Float|Clamp(Float) (- (Variables|Default|GetCurrentHealth) Damage) 0.0 1e+02)))
    (Default|CallEHealthUpdated _output_get (Variables|Default|GetMaxHealth))
    (if (== _output_get 0.0)
      (Development|PrintString "Dead")
      (Variables|Default|SetisDead true)
      (Components|Animation|PlayAnimation (Variables|Character|GetMesh) "/Game/Animations/Dying_Backwards.Dying_Backwards" false)
      (Input|DisableInput (Game|GetPlayerController 0)))))

(event EventBeginPlay
  (bind _fullauto (Variables|Default|GetFullAuto))
  ;[0.15 0.15 0.15 0.5] HealthUI
  (bind _returnvalue (UserInterface|CreateWidget "/Game/UI/WBP_HUD.WBP_HUD_C"))
  (UserInterface|Viewport|AddtoViewport _returnvalue 0)
  (Default|Initialise _returnvalue self)
  (Default|CallEHealthUpdated (Variables|Default|GetCurrentHealth) (Variables|Default|GetMaxHealth))
  (bind _returnvalue_2 (UserInterface|CreateWidget "/Game/UserWidget/AmmoCounter_UI.AmmoCounter_UI_C"))
  (UserInterface|Viewport|AddtoViewport _returnvalue_2 0)
  (Default|Setup _returnvalue_2 self)
  (Default|CallEAmmoUpdated (Math|Float|Truncate (Variables|/Game/Weapons/Weapons/BP_BaseWeapon.BP_BaseWeapon_C|GetAmmo _fullauto)) (Math|Float|Truncate (Variables|/Game/Weapons/Weapons/BP_BaseWeapon.BP_BaseWeapon_C|GetMaxAmmo _fullauto)))
  (bind _returnvalue_3 (Game|SpawnActorfromClass "/Game/Weapons/Weapons/BP_SemiAutoBaseWeapon.BP_SemiAutoBaseWeapon_C" (Transformation|GetActorTransform) "Undefined" "MultiplyWithRoot" 0 0))
  (bind _output_get (Variables|Default|SetEquippedWeapon _returnvalue_3))
  (Transformation|AttachComponentToComponent _output_get (Variables|Character|GetMesh) "WeaponSocket" "SnapToTarget" "SnapToTarget" "SnapToTarget" true))

(event EventTick
  (params (DeltaSeconds :type Float%20%28single-precision%29))
  ;[0.15 0.15 0.15 0.5] Camera
)

(event Input|MouseEvents|RightMouseButton
  (params (Key :type Key%20Structure :default "None"))
  ;[0.15 0.15 0.15 0.5] Aiming
  (:Pressed
    (Animation|Montage|PlayMontage (Variables|Character|GetMesh) "/Game/Animations/Rifle_Aiming_Idle_Montage.Rifle_Aiming_Idle_Montage"
      (:then
        (Variables|Default|SetAiming true)
        (bind _returnvalue (UserInterface|CreateWidget "/Game/UserWidget/Crosshair_UI.Crosshair_UI_C"))
        (UserInterface|Viewport|AddtoViewport _returnvalue 0))))
  (:Released
    (Animation|Montage|PlayMontage (Variables|Character|GetMesh) "/Game/Animations/Rifle_Aiming_Idle_Montage.Rifle_Aiming_Idle_Montage" 1.0 3.1
      (:then
        (Variables|Default|SetAiming false)
        (Widget|RemovefromParent _returnvalue)))))

(fn ConstructionScript)

(fn Sprint
  (Variables|/Script/Engine.CharacterMovementComponent|SetMaxWalkSpeed (Variables|Character|GetCharacterMovement) (Variables|Default|GetSprintSpeed)))

(fn StopSprinting
  (Variables|/Script/Engine.CharacterMovementComponent|SetMaxWalkSpeed (Variables|Character|GetCharacterMovement) (Variables|Default|GetWalkSpeed)))