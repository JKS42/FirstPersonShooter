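; BP_Enemy is a character Blueprint that holds both ragdoll hit reaction and left-mouse rifle shooting logic.
; HitImpact enables mesh physics and applies a directional velocity-change impulse to the given bone.
; While aiming, clicking plays montages, faces control rotation, shakes the camera and traces PhysicsBody objects from screen center.
; It then spawns BP_Bullet at the rifle, aimed at the trace point and carrying the hit bone name.
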(event Custom|BulletTrace
  (bind _returnvalue (Game|GetPlayerController 0))
  (bind (_sizex _sizey) (HUD|GetViewportSize _returnvalue))
  (bind _returnvalue_2 (/ _sizey 2))
  (bind _returnvalue_3 (/ _sizex 2))
  (bind _returnvalue_4 (Math|Conversions|ToFloat(Integer) _returnvalue_3))
  (bind _returnvalue_5 (Math|Conversions|ToFloat(Integer) _returnvalue_2))
  (bind (_worldlocation _worlddirection) (Class|PlayerController|DeprojectScreenPositiontoWorld _returnvalue _returnvalue_4 _returnvalue_5))
  ;[0.15 0.15 0.15 0.5] HitTrace
  (bind (_outhit _returnvalue_6) (Collision|LineTraceForObjects (+ _worldlocation (* _worlddirection 1e+01)) (+ _worldlocation (* _worlddirection 3e+03)) (Utilities|Array|MakeArray "ObjectTypeQuery4") false 0 "ForDuration"))
  (if _returnvalue_6
    (Variables|Default|SetBulletImpactLoc (.ImpactPoint (Collision|BreakHitResult _outhit)))
    (bind _output_get (Variables|Default|SetHitBoneName (.HitBoneName (Collision|BreakHitResult _outhit))))
    (Development|PrintText (Utilities|Text|ToText(Name) _output_get))
    (else
      (Variables|Default|SetBulletImpactLoc (.TraceEnd (Collision|BreakHitResult _outhit))))))

(event Custom|HitImpact
  (params (ForwardVector :type Vector) (RightVector :type Vector) (Impulse%20AMT :type Float%20%28double-precision%29) (Bone%20Name :type Name))
  (bind _mesh (Variables|Character|GetMesh))
  (Collision|SetCollisionEnabled _mesh "QueryAndPhysics")
  (Physics|SetSimulatePhysics _mesh true)
  (Physics|AddImpulse (Variables|Character|GetMesh) (* (Math|Vector|RotateVector ForwardVector (Math|Vector|RotatorfromAxisandAngle (Math|Vector|NegateVector RightVector) 0.0)) Impulse%20AMT) Bone%20Name true))

(event Input|MouseEvents|LeftMouseButton
  (params (Key :type Key%20Structure :default "None"))
  (bind _mesh (Variables|Character|GetMesh))
  (bind _assaultrifle (Variables|Default|GetAssaultRifle))
  (bind _returnvalue (Transformation|GetWorldLocation _assaultrifle))
  ;[0.15 0.15 0.15 0.5] Shooting
  (:Pressed
    (if (Variables|Default|GetAiming)
      (Utilities|FlowControl|Sequence
        (:then_0
          (Animation|Montage|PlayMontage _mesh "/Game/Animations/Firing_Rifle_Montage.Firing_Rifle_Montage"
            (:then
              (Utilities|FlowControl|Delay 1.17))
            (:OnBlendOut
              (Animation|Montage|PlayMontage _mesh "/Game/Animations/Rifle_Aiming_Idle_Montage.Rifle_Aiming_Idle_Montage" 0.0))))
        (:then_1
          (Transformation|SetActorRotation (Pawn|GetControlRotation :!class /Script/Engine.Pawn))
          (Camera|PlayWorldCameraShake "/Game/Blueprints/BP_CameraShake.BP_CameraShake_C" (Transformation|GetActorLocation) 0.0 1e+03)
          (CallFunction|BulletTrace)
          (bind _returnvalue_2 (Game|SpawnActorfromClass "/Game/Blueprints/BP_Bullet.BP_Bullet_C" (Math|Transform|MakeTransform _returnvalue (Math|Rotator|FindLookatRotation _returnvalue (Variables|Default|GetBulletImpactLoc)) "1.000000,1.000000,1.000000") "Undefined" "MultiplyWithRoot" 0 0))
          (bind _output_get (Variables|Default|SetBulletRef _returnvalue_2))
          (Variables|/Game/Blueprints/BP_Bullet.BP_Bullet_C|SetBoneName _output_get (Variables|Default|GetHitBoneName)))))))

(fn ConstructionScript)