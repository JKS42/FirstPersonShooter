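; BP_Enemy3 is a ranged enemy with a widget health bar that faces any BP_BaseCharacter it sees.
; Pawn sensing triggers a cooldown-gated attack that spawns a projectile and also applies damage directly to the seen character.
; Damage and healing update the health widget; at zero health it calls the first BP_OnDeath actor's death event and destroys itself.
; Its destruction asks BP_Game to respawn an enemy.
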(event OnSeePawn(PawnSensing)
  (params (Pawn :type Pawn%20Object%20Reference))
  (bind _asbp_base_character (Utilities|Casting|CastToBP_BaseCharacter Pawn))
  (Transformation|SetActorRotation (Math|Rotator|FindRelativeLookatRotation (Math|Conversions|ToTransform(Vector) (Transformation|GetActorLocation)) (Transformation|GetActorLocation _asbp_base_character)))
  (if (Variables|Default|GetCanAttack?)
    (Game|SpawnActorfromClass "/Game/Enemy/BP_EnemyProjectile.BP_EnemyProjectile_C" (Transformation|GetWorldTransform (Variables|Default|GetSpawn)) "Undefined" "MultiplyWithRoot" 0 0)
    (Game|Damage|ApplyDamage _asbp_base_character 3.0 0 0)
    (Variables|Default|SetCanAttack? false)
    (Utilities|FlowControl|Delay 0.5)
    (Variables|Default|SetCanAttack? true)))

(event EventBeginPlay
  (bind _aswbp_enemy_health (Utilities|Casting|CastToWBP_EnemyHealth (UserInterface|GetUserWidgetObject (Variables|Default|GetWidget))))
  (bind _output_get (Variables|Default|SetWBP%20Enemy%20Health _aswbp_enemy_health))
  (Variables|/Game/Enemy/WBP_EnemyHealth.WBP_EnemyHealth_C|SetCurrentHealth _output_get (Variables|Default|GetCurrentHealth))
  (Variables|/Game/Enemy/WBP_EnemyHealth.WBP_EnemyHealth_C|SetMaxHealth _output_get (Variables|Default|GetMaxHealth)))

(event Game|Damage|EventAnyDamage
  (params (Damage :type Float%20%28single-precision%29) (DamageType :type Damage%20Type%20Object%20Reference) (InstigatedBy :type Controller%20Object%20Reference) (DamageCauser :type Actor%20Object%20Reference))
  ;[0.15 0.15 0.15 0.5] DamageTaken
  (bind _output_get (Variables|Default|SetCurrentHealth (Math|Float|Truncate (- (Variables|Default|GetCurrentHealth) Damage))))
  (Default|UpdateHealth (Variables|Default|GetWBP%20Enemy%20Health) _output_get)
  (if (<= _output_get 0)
    (bind _outactors (Actor|GetAllActorsOfClass "/Game/Blueprints/BP_OnDeath.BP_OnDeath_C"))
    (Default|CallOnDeathEvent (Utilities|Array|Get(acopy) _outactors))
    (Actor|DestroyActor)))

(event EventDestroyed
  ;[0.15 0.15 0.15 0.5] Respawn
  (bind _asbp_game (Utilities|Casting|CastToBP_Game (Game|GetGameMode)))
  (Default|RespawnEnemy _asbp_game))

(event EventHeal
  (params (HealAmount :type Float%20%28double-precision%29) (MaxHealth :type Float%20%28double-precision%29))
  ;[0.15 0.15 0.15 0.5] HealthPickup
  (bind _output_get (Variables|Default|SetCurrentHealth (+ HealAmount (Variables|Default|GetCurrentHealth))))
  (if (>= _output_get MaxHealth)
    (bind _output_get_2 (Variables|Default|SetCurrentHealth (Variables|Default|GetMaxHealth)))
    (Default|UpdateHealth (Variables|Default|GetWBP%20Enemy%20Health) _output_get_2)
    (else
      (Default|UpdateHealth (Variables|Default|GetWBP%20Enemy%20Health) _output_get))))

(fn ConstructionScript)