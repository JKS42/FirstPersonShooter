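; Full-auto base weapon Blueprint that fires repeated trace shots while shooting is active.
; Shoot calls the parent, then starts a looping timer at the FireRate interval, stored in Timer.
; Each timer tick runs FullAutoShoot, which performs a ShotTrace over Range.
; EndShoot calls the parent and clears the timer to stop firing.
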(event Custom|FullAutoShoot
  (CallFunction|ShotTrace (Variables|Default|GetRange)))

(event EventShoot
  (|CallParentFunction)
  (bind _returnvalue (Utilities|Time|SetTimerbyEvent (delegate Custom|FullAutoShoot) (Variables|Default|GetFireRate) true))
  (Variables|Default|SetTimer _returnvalue))

(event EventEndShoot
  (|CallParentFunction)
  (Utilities|Time|ClearandInvalidateTimerbyHandle (Variables|Default|GetTimer)))

(fn ConstructionScript
  (|CallParentFunction))