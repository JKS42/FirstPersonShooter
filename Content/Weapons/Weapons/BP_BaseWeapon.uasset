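; BP_BaseWeapon is a base weapon Blueprint that provides hitscan firing, with empty Shoot and EndShoot events.
; ShotTrace spends one round, then line-traces forward from ShootArrow over the given Range and applies Damage to every Pawn hit returned.
; With no ammo left, it still fires if Infinite is set.
; The trace draws timed debug lines.
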(event Custom|ShotTrace
  (params (Range :type Float%20%28double-precision%29))
  (bind _shootarrow (Variables|Default|GetShootArrow))
  (bind _returnvalue (Transformation|GetWorldLocation _shootarrow))
  (if (> (Variables|Default|GetAmmo) 0.0)
    (Variables|Default|SetAmmo (- (Variables|Default|GetAmmo) 1.0))
    (bind (_outhits _returnvalue_2) (Class|KismetSystemLibrary|LineTraceMultiforObjects _returnvalue (+ _returnvalue (* (Math|Vector|GetForwardVector (Transformation|GetWorldRotation _shootarrow)) Range)) (Utilities|Array|MakeArray "ObjectTypeQuery3") false 0 "ForDuration" true :!label _label))
    (if _returnvalue_2
      (bind _array_element (Utilities|Array|ForEachLoopwithBreak _outhits)
        (:LoopBody
          (Game|Damage|ApplyDamage (.HitActor (Collision|BreakHitResult _array_element)) (Variables|Default|GetDamage) 0 0))))
    (elif (Variables|Default|GetInfinite)
      (goto _label))))

(event Custom|Shoot)

(event Custom|EndShoot)

(fn ConstructionScript)